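; Breakable statue target that swaps its static mesh for a Chaos Geometry Collection when hit or damaged.
; A sufficiently strong hit sets a one-time broken flag, hides the mesh, then applies strain and a radial impulse to shatter the collection.
; Any positive damage only performs the swap, without checking or setting the flag.
; Break events disable collision on the broken piece and the original mesh.
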(event `self.ReceiveHit`
  (params (MyComp :type "PrimitiveComponent Object Reference") (Other :type "Actor Object Reference") (OtherComp :type "PrimitiveComponent Object Reference") (bSelfMoved :type Boolean) (HitLocation :type "Vector Structure") (HitNormal :type "Vector Structure") (NormalImpulse :type "Vector Structure") (Hit :type "HitResult Structure (by ref)"))
  (if (`self.IsBroken`)
    _
    (elif (>= (`KismetMathLibrary.VSize` NormalImpulse) 30000.0)
      (set `self.IsBroken` true)
      (`SceneComponent.SetVisibility` (`self.StaticMesh`) false false)
      (`PrimitiveComponent.SetSimulatePhysics` (`self.StaticMesh`) false)
      (`GeometryCollectionComponent.SetRestCollection` (`self.GeometryCollection`) "/Game/StarterContent/Props/SM_Statue_SM_Statue/GC_SM_Statue.GC_SM_Statue" true)
      (`GeometryCollectionComponent.ApplyExternalStrain` (`self.GeometryCollection`) 0 HitLocation 100.0 1 1.0 500000.0)
      (`PrimitiveComponent.AddRadialImpulse` (`self.GeometryCollection`) (`self.K2_GetActorLocation`) 100.0 200.0 "RIF_Constant" false)
      (`PrimitiveComponent.SetWalkableSlopeOverride` (`self.GeometryCollection`) (make `WalkableSlopeOverride` "WalkableSlope_Unwalkable")))))

(event `self.ReceiveBeginPlay`
  (add `self.OnTakeAnyDamage` (delegate `CE_TakeAnyDamage`)))

(event `CE_TakeAnyDamage` :!signature `self.OnTakeAnyDamage`
  (params (DamagedActor :type "Actor Object Reference") (Damage :type "Float (single-precision)") (DamageType :type "DamageType Object Reference") (InstigatedBy :type "Controller Object Reference") (DamageCauser :type "Actor Object Reference"))
  (if (> Damage 0.0)
    (`SceneComponent.SetVisibility` (`self.StaticMesh`) false false)
    (`PrimitiveComponent.SetSimulatePhysics` (`self.StaticMesh`) false)
    (`GeometryCollectionComponent.SetRestCollection` (`self.GeometryCollection`) "/Game/StarterContent/Props/SM_Statue_SM_Statue/GC_SM_Statue.GC_SM_Statue" true)))

(event `self.GeometryCollection.OnChaosBreakEvent`
  (params (BreakEvent :type "ChaosBreakEvent Structure (by ref)"))
  (`GeometryCollectionComponent.SetPerParticleCollisionProfileName` (`self.GeometryCollection`) (`|MakeArray` BreakEvent_Index) "None")
  (`PrimitiveComponent.SetCollisionEnabled` (`self.StaticMesh`) "NoCollision"))

(fn `UserConstructionScript`)